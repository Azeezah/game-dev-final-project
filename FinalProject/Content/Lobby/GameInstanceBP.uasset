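; Game instance Blueprint that rotates the game through its list of minigames.
; LaunchNextGame takes the entry after CurrentMinigame from GetMinigames, wrapping around or starting at the first when the current one is not listed.
; It stores that entry and travels to it through a ServerTravel console command.
; An authority check with widget removal and a listen-server OpenLevel call are left unconnected.
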(fn `LaunchNextGame`
  (params (Target :type "Actor Object Reference"))
  (bind _minigames (`/Game/Lobby/CharacterFunctionLibrary.GetMinigames`))
  (bind _output_get (set `self.currentMinigame` (`|GetArrayItem` _minigames (mod (+ (`KismetArrayLibrary.Array_Find` _minigames (`self.currentMinigame`)) 1) (`KismetArrayLibrary.Array_Length` _minigames)))))
  (`KismetSystemLibrary.ExecuteConsoleCommand` (`KismetStringLibrary.Concat_StrStr` "ServerTravel " _output_get) null))